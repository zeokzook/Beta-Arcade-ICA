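; GlobalVariables holds copies of EvilBun player state (health, mana, power-up staff and score) so it can be saved and restored.
; SaveVariables reads these values from the EvilBunCharacter and EvilBunController into its global variables, and LoadVariables writes them back.
; Both functions find their targets with GetActorOfClass and use the results without validity checks.
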(fn SaveVariables
  (Utilities|FlowControl|Sequence
    (:then_0
      (bind _returnvalue (Actor|GetActorOfClass "/Game/Character/EvilBunCharacter.EvilBunCharacter_C"))
      (Variables|Default|SetGlobalHealth (Variables|/Game/Character/EvilBunCharacter.EvilBunCharacter_C|GetHealthPoints _returnvalue))
      (Variables|Default|SetGlobalMana (Variables|/Game/Character/EvilBunCharacter.EvilBunCharacter_C|GetcurrentMana _returnvalue))
      (Variables|Default|SetSecondary%20Weapon (Variables|/Game/Character/EvilBunCharacter.EvilBunCharacter_C|GetPowerUpStaff _returnvalue)))
    (:then_1
      (bind _returnvalue_2 (Actor|GetActorOfClass "/Game/Character/EvilBunController.EvilBunController_C"))
      (Variables|Default|SetGlobal%20Score (Variables|/Game/Character/EvilBunController.EvilBunController_C|GetScore _returnvalue_2)))))

(fn LoadVariables
  (Utilities|FlowControl|Sequence
    (:then_0
      (bind _returnvalue (Actor|GetActorOfClass "/Game/Character/EvilBunCharacter.EvilBunCharacter_C"))
      (Variables|/Game/Character/EvilBunCharacter.EvilBunCharacter_C|SetHealthPoints _returnvalue (Variables|Default|GetGlobalHealth))
      (Variables|/Game/Character/EvilBunCharacter.EvilBunCharacter_C|SetcurrentMana _returnvalue (Variables|Default|GetGlobalMana))
      (Variables|/Game/Character/EvilBunCharacter.EvilBunCharacter_C|SetPowerUpStaff _returnvalue (Variables|Default|GetSecondary%20Weapon)))
    (:then_1
      (bind _returnvalue_2 (Actor|GetActorOfClass "/Game/Character/EvilBunController.EvilBunController_C"))
      (Variables|/Game/Character/EvilBunController.EvilBunController_C|SetScore _returnvalue_2 (Variables|Default|GetGlobal%20Score)))))