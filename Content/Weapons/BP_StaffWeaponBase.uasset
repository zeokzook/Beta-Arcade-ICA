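; Base staff weapon for the EvilBun player character, providing mana-gated primary and optional secondary fire.
; Shoot events check mana, deduct the cost, then call effect hooks, with empty functions presumably left for child staffs to override.
; Helpers not called here offer three attack styles: muzzle-spawned projectile, line-trace stream, and a sphere on the player's AOE socket that expands on activation.
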(event Custom|OnShoot
  (params (CrosshairLocation :type Vector))
  (Variables|Default|SetCrosshairLocation CrosshairLocation)
  (bind _canshoot (CallFunction|CanShoot))
  (if _canshoot
    (CallFunction|DecreaseMana)
    (CallFunction|PlayEffects)
    (CallFunction|PlayShootSounds)
    (else
      (CallFunction|PlayNoManaSounds))))

(event Custom|onSecondaryShoot
  (params (CrosshairLocation :type Vector))
  (Variables|Default|SetCrosshairLocation CrosshairLocation)
  (if (Variables|Default|GethaveSecondary)
    (Variables|Default|SetSecondary? true)
    (bind _canshoot (CallFunction|CanShoot))
    (if _canshoot
      (CallFunction|DecreaseMana)
      (CallFunction|PlayEffects)
      (else
        (CallFunction|PlayNoManaSounds)))))

(event EventBeginPlay
  (bind _asevil_bun_character (Utilities|Casting|CastToEvilBunCharacter (Game|GetPlayerCharacter 0)))
  (Variables|Default|SetPlayer _asevil_bun_character)
  (Transformation|AttachComponentToComponent (Variables|Default|GetSphere) (Variables|/Game/Character/EvilBunCharacter.EvilBunCharacter_C|GetAOESocket _asevil_bun_character) "None" "KeepRelative" "KeepRelative" "KeepRelative" true)
  (Components|Sphere|SetSphereRadius (Variables|Default|GetSphere) 0.0 false))

(fn ConstructionScript)

(fn CanShoot
  (bind _player (Variables|Default|GetPlayer))
  (if (Variables|/Game/Character/EvilBunCharacter.EvilBunCharacter_C|GetInfiniteMana? _player)
    _
    (elif (== (Variables|Default|GetprimaryManaCost) 0.0)
      _
      (elif (== (Variables|Default|GetsecondaryManaCost) 0.0)
        _
        (elif (> (Variables|/Game/Character/EvilBunCharacter.EvilBunCharacter_C|GetcurrentMana _player) 0.0)
          _
          (else
            (Development|PrintString "Out of Mana!" true true "(R=0.000000,G=0.660000,B=1.000000,A=1.000000)" 1.0)
            (Variables|Default|SetcanShoot? false)
            (return false))))))
  (Variables|Default|SetcanShoot? true)
  (return true))

(fn DecreaseMana
  (bind _player (Variables|Default|GetPlayer))
  (if (not (Variables|/Game/Character/EvilBunCharacter.EvilBunCharacter_C|GetInfiniteMana? _player))
    (if (Variables|Default|GetSecondary?)
      (bind _output_get (Variables|/Game/Character/EvilBunCharacter.EvilBunCharacter_C|SetcurrentMana _player (Math|Float|Clamp(Float) (- (Variables|/Game/Character/EvilBunCharacter.EvilBunCharacter_C|GetcurrentMana _player) (Variables|Default|GetsecondaryManaCost)) 0.0 (Variables|/Game/Character/EvilBunCharacter.EvilBunCharacter_C|GetmaxMana _player))))
      (Variables|Default|SetSecondary? false)
      (Development|PrintString (Utilities|String|BuildString(Float) "" "Current Mana: " _output_get) true true "(R=0.000000,G=0.660000,B=1.000000,A=1.000000)" 1.0)
      (elif (not (== (Variables|Default|GetprimaryManaCost) 0.0))
        (bind _output_get_2 (Variables|/Game/Character/EvilBunCharacter.EvilBunCharacter_C|SetcurrentMana _player (Math|Float|Clamp(Float) (- (Variables|/Game/Character/EvilBunCharacter.EvilBunCharacter_C|GetcurrentMana _player) (Variables|Default|GetprimaryManaCost)) 0.0 (Variables|/Game/Character/EvilBunCharacter.EvilBunCharacter_C|GetmaxMana _player))))
        (Development|PrintString (Utilities|String|BuildString(Float) "" "Current Mana: " _output_get_2) true true "(R=0.000000,G=0.660000,B=1.000000,A=1.000000)" 1.0)))))

(fn PlayEffects)

(fn PlayShootSounds
  (Audio|PlaySound2D "/Game/Sounds/Normal_shot.Normal_shot" 1.0 1.0 0.0 0 0))

(fn PlayNoManaSounds)

(fn ShootProjectile
  (bind _asevil_bun_character (Utilities|Casting|CastToEvilBunCharacter (Game|Player|GetPlayerPawn 0))
    (:then
      (CallFunction|SpawningProjectile (Math|Transform|MakeTransform (Transformation|GetWorldLocation (Variables|/Game/Character/EvilBunCharacter.EvilBunCharacter_C|GetMuzzle _asevil_bun_character)) (Transformation|GetWorldRotation (Variables|/Game/Character/EvilBunCharacter.EvilBunCharacter_C|GetMuzzle _asevil_bun_character)))))
    (:CastFailed
      (Development|PrintString "Player Cast Failed!"))))

(fn SpawningProjectile
  (params (spawnTransform :type Transform))
  (bind _returnvalue (Game|SpawnActorfromClass "/Game/Weapons/BP_ProjectileBase.BP_ProjectileBase_C" spawnTransform "Undefined" self 1e+01 (Game|GetInstigator)))
  (Variables|/Game/Weapons/BP_ProjectileBase.BP_ProjectileBase_C|SetBaseDamage _returnvalue (Variables|Default|GetbaseDamage)))

(fn ShootStream
  (bind _asevil_bun_character (Utilities|Casting|CastToEvilBunCharacter (Game|Player|GetPlayerPawn 0))
    (:then
      (CallFunction|PlayStreamEffects)
      (bind _outhit (Collision|LineTraceForObjects (Transformation|GetWorldLocation (Variables|/Game/Character/EvilBunCharacter.EvilBunCharacter_C|GetMuzzle _asevil_bun_character)) (+ (Transformation|GetWorldLocation (Variables|/Game/Character/EvilBunCharacter.EvilBunCharacter_C|GetMuzzle _asevil_bun_character)) (Class|KismetMathLibrary|CreateVectorfromYawPitch (.yaw (Transformation|GetWorldRotation (Variables|/Game/Character/EvilBunCharacter.EvilBunCharacter_C|GetMuzzle _asevil_bun_character))) (.pitch (Transformation|GetWorldRotation (Variables|/Game/Character/EvilBunCharacter.EvilBunCharacter_C|GetMuzzle _asevil_bun_character))) (Variables|Default|GetRange))) (Utilities|Array|MakeArray "ObjectTypeQuery3") false 0 "ForDuration" true "(R=1.000000,G=0.000000,B=0.000000,A=1.000000)" "(R=0.000000,G=1.000000,B=0.000000,A=1.000000)" 0.5))
      (Variables|Default|SetLastHitActor (.HitActor (Collision|BreakHitResult _outhit)))
      (return _outhit))
    (:CastFailed
      (Development|PrintString "Player Cast Failed!"))))

(fn PlayStreamEffects)

(fn ActivateAOE
  (Components|Sphere|SetSphereRadius (Variables|Default|GetSphere) (Variables|Default|GetAreaOfEffectSize) true))