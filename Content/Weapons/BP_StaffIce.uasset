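; Ice staff weapon that adds a projectile shot and a freezing stream on top of its parent's shooting logic.
; Primary fire, when allowed, shoots BP_ProjectileIce, spawned with the staff's damage, crosshair target and slow radius and despawn settings.
; Secondary fire passes the stream's hit to IceStream, which damages any BP_CollisionBase actor hit and calls its Freezing function.
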(event EventOnSecondaryShoot
  (params (CrosshairLocation :type Vector :default "0, 0, 0"))
  (|CallParentFunction CrosshairLocation)
  (if (Variables|Default|GetcanShoot?)
    (bind _hit_results (CallFunction|ShootStream))
    (CallFunction|IceStream _hit_results)))

(event EventOnShoot
  (params (CrosshairLocation :type Vector :default "0, 0, 0"))
  (|CallParentFunction CrosshairLocation)
  (if (Variables|Default|GetcanShoot?)
    (CallFunction|ShootProjectile)))

(fn ConstructionScript
  (|CallParentFunction))

(fn SpawningProjectile
  (params (spawnTransform :type Transform))
  (Game|SpawnActorfromClass "/Game/Weapons/BP_ProjectileIce.BP_ProjectileIce_C" spawnTransform "Undefined" self (Variables|Default|GetslowRadius) (Variables|Default|GetslowDespawnTimer) (Variables|Default|GetCrosshairLocation) (Variables|Default|GetbaseDamage) (Game|GetInstigator)))

(fn IceStream
  (params (Hit :type Hit%20Result%20Structure))
  (bind _hitactor (Collision|BreakHitResult Hit))
  (bind _asbp_collision_base (Utilities|Casting|CastToBP_CollisionBase _hitactor))
  (Game|Damage|ApplyDamage _asbp_collision_base (Variables|Default|GetbaseDamage) (Game|GetInstigatorController) 0)
  (Utilities|IsValid _hitactor
    (:Is%20Valid
      (Default|Freezing _asbp_collision_base))))