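; Ice projectile that turns into a lingering slow and damage-over-time area near the crosshair's target point.
; Each tick it compares distance travelled to the player-to-crosshair distance minus an offset, then stops, hides its mesh, expands the zero-radius collision sphere and turns on the ice effect and light.
; Sphere overlaps start slow and ice damage on BP_CollisionBase actors and clear both on exit.
; The actor destroys itself after a timer started at spawn.
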(event OnComponentHit(CollisionSphere)
  (params (HitComponent :type Primitive%20Component%20Object%20Reference) (OtherActor :type Actor%20Object%20Reference) (OtherComp :type Primitive%20Component%20Object%20Reference) (NormalImpulse :type Vector :default "0, 0, 0") (Hit :type Hit%20Result%20Structure%20%28by%20ref%29)))

(event OnComponentBeginOverlap(CollisionSphere)
  (params (OverlappedComponent :type Primitive%20Component%20Object%20Reference) (OtherActor :type Actor%20Object%20Reference) (OtherComp :type Primitive%20Component%20Object%20Reference) (OtherBodyIndex :type Integer) (bFromSweep :type Boolean) (SweepResult :type Hit%20Result%20Structure%20%28by%20ref%29))
  (bind _asbp_collision_base (Utilities|Casting|CastToBP_CollisionBase OtherActor))
  (Default|Slow _asbp_collision_base)
  (Default|OnDoT _asbp_collision_base (Variables|Default|GetBaseDamage) 1e+01 false true))

(event OnComponentEndOverlap(CollisionSphere)
  (params (OverlappedComponent :type Primitive%20Component%20Object%20Reference) (OtherActor :type Actor%20Object%20Reference) (OtherComp :type Primitive%20Component%20Object%20Reference) (OtherBodyIndex :type Integer))
  (bind _asbp_collision_base (Utilities|Casting|CastToBP_CollisionBase OtherActor))
  (Default|EndSlow _asbp_collision_base)
  (Default|NotonDoT _asbp_collision_base))

(event EventTick
  (params (DeltaSeconds :type Float%20%28single-precision%29))
  (bind _projectilemovement (Variables|Default|GetProjectileMovement))
  (if (>= (Math|Vector|Distance(Vector) (Variables|Default|GetinitLocation) (Transformation|GetActorLocation)) (- (Math|Vector|Distance(Vector) (Variables|Default|GetcrosshairLocation) (Transformation|GetActorLocation (Game|GetPlayerCharacter 0))) 1.3e+02))
    (Components|Sphere|SetSphereRadius (Variables|Default|GetCollisionSphere) (Variables|Default|GetsphereRadius) true)
    (Game|Components|ProjectileMovement|SetVelocityinLocalSpace _projectilemovement "0, 0, 0")
    (Variables|/Script/Engine.ProjectileMovementComponent|SetProjectileGravityScale _projectilemovement 0.0)
    (Development|SetHiddeninGame (Variables|Default|GetSphere) true false)
    (Components|Activation|Activate (Variables|Default|GetIceArea) false)
    (Rendering|Components|Light|SetIntensity (Variables|Default|GetSpotLight) 1e+05)))

(event EventBeginPlay
  (|CallParentFunction)
  (Components|Sphere|SetSphereRadius (Variables|Default|GetCollisionSphere) 0.0 true)
  (Variables|Default|SetinitLocation (Transformation|GetActorLocation))
  (Components|Activation|Deactivate (Variables|Default|GetIceArea))
  (Rendering|Components|Light|SetIntensity (Variables|Default|GetSpotLight) 0.0)
  (Utilities|FlowControl|Delay (Variables|Default|GetdespawnTimer))
  (Actor|DestroyActor))

(fn ConstructionScript
  (|CallParentFunction))