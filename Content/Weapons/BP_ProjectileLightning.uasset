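; BP_ProjectileLightning is a lightning projectile that damages whatever actor its collision sphere hits.
; On hit it applies base damage credited to the instigator's controller, using the fire damage type despite the lightning theme.
; If the hit actor is a BP_CollisionBase it also calls that actor's Electric function with the same damage, then the projectile destroys itself.
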(event OnComponentHit(CollisionSphere)
  (params (HitComponent :type Primitive%20Component%20Object%20Reference) (OtherActor :type Actor%20Object%20Reference) (OtherComp :type Primitive%20Component%20Object%20Reference) (NormalImpulse :type Vector :default "0, 0, 0") (Hit :type Hit%20Result%20Structure%20%28by%20ref%29))
  (Game|Damage|ApplyDamage OtherActor (Variables|Default|GetBaseDamage) (Game|GetInstigatorController) self "/Game/Weapons/DamageTypes/DmgType_Fire.DmgType_Fire_C")
  (bind _asbp_collision_base (Utilities|Casting|CastToBP_CollisionBase OtherActor)
    (:then
      (Utilities|IsValid _asbp_collision_base
        (:Is%20Valid
          (Default|Electric _asbp_collision_base 0 (Variables|Default|GetBaseDamage) 0 false))
        (:Is%20Not%20Valid
          _)))
    (:CastFailed
      _))
  (Actor|DestroyActor))

(fn ConstructionScript
  (|CallParentFunction))