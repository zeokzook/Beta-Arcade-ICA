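; BP_ProjectileBase is a base projectile Blueprint that deals damage to what it hits.
; On BeginPlay it applies the ProjectileSpeed variable to the projectile movement component as local forward velocity, initial speed and max speed.
; A CollisionSphere hit applies BaseDamage with DmgType_Basic, credited to the instigator's controller, calls PlayEffects and destroys the actor.
; PlayEffects is empty in this class.
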(event OnComponentHit(CollisionSphere)
  (params (HitComponent :type Primitive%20Component%20Object%20Reference) (OtherActor :type Actor%20Object%20Reference) (OtherComp :type Primitive%20Component%20Object%20Reference) (NormalImpulse :type Vector :default "0, 0, 0") (Hit :type Hit%20Result%20Structure%20%28by%20ref%29))
  (Game|Damage|ApplyDamage OtherActor (Variables|Default|GetBaseDamage) (Game|GetInstigatorController) self "/Game/Weapons/DamageTypes/DmgType_Basic.DmgType_Basic_C")
  (CallFunction|PlayEffects)
  (Actor|DestroyActor))

(event EventBeginPlay
  (bind _projectilemovement (Variables|Default|GetProjectileMovement))
  (bind _projectilespeed (Variables|Default|GetProjectileSpeed))
  ;[1 1 1] Setting Initial Speed, editable at under variables (on the left)
  (Game|Components|ProjectileMovement|SetVelocityinLocalSpace _projectilemovement (Math|Vector|MakeVector _projectilespeed 0.0 0.0))
  (bind _output_get (Variables|/Script/Engine.ProjectileMovementComponent|SetInitialSpeed _projectilemovement _projectilespeed))
  (Variables|/Script/Engine.ProjectileMovementComponent|SetMaxSpeed _projectilemovement _output_get))

(fn ConstructionScript)

(fn PlayEffects)