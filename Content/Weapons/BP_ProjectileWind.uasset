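; Wind projectile that flies forward, stops near the crosshair's target distance and stuns BP_CollisionBase actors that overlap its sphere.
; BeginPlay sets speed and sphere radius, records the spawn location and destroys the actor after DespawnTimer.
; Tick halts movement and gravity once travel reaches the player-to-crosshair distance, less a fixed offset.
; Stun calls receive the full DespawnTimer, regardless of remaining lifetime; PlayEffects is empty.
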(event OnComponentBeginOverlap(CollisionSphere)
  (params (OverlappedComponent :type Primitive%20Component%20Object%20Reference) (OtherActor :type Actor%20Object%20Reference) (OtherComp :type Primitive%20Component%20Object%20Reference) (OtherBodyIndex :type Integer) (bFromSweep :type Boolean) (SweepResult :type Hit%20Result%20Structure%20%28by%20ref%29))
  (bind _asbp_collision_base (Utilities|Casting|CastToBP_CollisionBase OtherActor))
  (Default|Stunned _asbp_collision_base (Variables|Default|GetdespawnTimer)))

(event EventBeginPlay
  (bind _projectilemovement (Variables|Default|GetProjectileMovement))
  (bind _projectilespeed (Variables|Default|GetprojectileSpeed))
  (Game|Components|ProjectileMovement|SetVelocityinLocalSpace _projectilemovement (Math|Vector|MakeVector _projectilespeed 0.0 0.0))
  (bind _output_get (Variables|/Script/Engine.ProjectileMovementComponent|SetInitialSpeed _projectilemovement _projectilespeed))
  (Variables|/Script/Engine.ProjectileMovementComponent|SetMaxSpeed _projectilemovement _output_get)
  (Components|Sphere|SetSphereRadius (Variables|Default|GetCollisionSphere) (Variables|Default|GetsphereRadius) true)
  (Variables|Default|SetinitLocation (Transformation|GetActorLocation))
  (Utilities|FlowControl|Delay (Variables|Default|GetdespawnTimer))
  (Actor|DestroyActor))

(event EventTick
  (params (DeltaSeconds :type Float%20%28single-precision%29))
  (bind _projectilemovement (Variables|Default|GetProjectileMovement))
  (if (>= (Math|Vector|Distance(Vector) (Variables|Default|GetinitLocation) (Transformation|GetActorLocation)) (- (Math|Vector|Distance(Vector) (Variables|Default|GetcrosshairLocation) (Transformation|GetActorLocation (Game|GetPlayerCharacter 0))) 1.3e+02))
    (Game|Components|ProjectileMovement|SetVelocityinLocalSpace _projectilemovement "0, 0, 0")
    (Variables|/Script/Engine.ProjectileMovementComponent|SetProjectileGravityScale _projectilemovement 0.0)))

(fn ConstructionScript)

(fn PlayEffects)