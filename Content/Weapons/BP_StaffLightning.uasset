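; Lightning staff weapon that fires lightning projectiles as its primary attack and a chaining electric stream as its secondary.
; Primary fire calls the parent's ShootProjectile, with SpawningProjectile supplying BP_ProjectileLightning.
; Secondary fire passes the ShootStream hit to LightningStream, which damages BP_CollisionBase targets and triggers their chained Electric effect.
; The struck target shows an electric beam for one second.
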(event EventOnShoot
  (params (CrosshairLocation :type Vector :default "0, 0, 0"))
  (|CallParentFunction "0, 0, 0")
  (if (Variables|Default|GetcanShoot?)
    (CallFunction|ShootProjectile)))

(event EventOnSecondaryShoot
  (params (CrosshairLocation :type Vector :default "0, 0, 0"))
  (|CallParentFunction "0, 0, 0")
  (if (Variables|Default|GetcanShoot?)
    (bind _hit_results (CallFunction|ShootStream))
    (bind _collisionbase (CallFunction|LightningStream _hit_results))
    (Utilities|IsValid _collisionbase
      (:Is%20Valid
        (Default|BeginElectricBeam _collisionbase)
        (Utilities|FlowControl|Delay 1.0)
        (Utilities|IsValid _collisionbase
          (:Is%20Valid
            (Default|EndElectricBeam _collisionbase)))))))

(fn ConstructionScript
  (|CallParentFunction))

(fn SpawningProjectile
  (params (spawnTransform :type Transform))
  (Game|SpawnActorfromClass "/Game/Weapons/BP_ProjectileLightning.BP_ProjectileLightning_C" spawnTransform "Undefined" self (Variables|Default|GetbaseDamage) (Game|GetInstigator)))

(fn LightningStream
  (params (Hit%20Results :type Hit%20Result%20Structure))
  (bind _lightningstreamdamage (Variables|Default|GetLightningStreamDamage))
  (bind _asbp_collision_base (Utilities|Casting|CastToBP_CollisionBase (.HitActor (Collision|BreakHitResult Hit%20Results))))
  (Game|Damage|ApplyDamage _asbp_collision_base _lightningstreamdamage (Game|GetInstigatorController) self)
  (Utilities|IsValid _asbp_collision_base
    (:Is%20Valid
      (Default|Electric _asbp_collision_base 0 _lightningstreamdamage 0 true)
      (return _asbp_collision_base))))