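; Wind staff weapon that fires hurricane projectiles on primary shoot and triggers an area knockback on secondary shoot.
; Both shots run parent logic and check CanShoot; the projectile spawn passes hurricane range, despawn timer and crosshair location to BP_ProjectileWind.
; The AOE calls Knockback on BP_CollisionBase actors overlapping the sphere, using player 0's location, then zeroes the sphere radius without updating overlaps.
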(event EventOnSecondaryShoot
  (params (CrosshairLocation :type Vector :default "0, 0, 0"))
  (|CallParentFunction CrosshairLocation)
  (if (Variables|Default|GetcanShoot?)
    (CallFunction|ActivateAOE)))

(event EventOnShoot
  (params (CrosshairLocation :type Vector :default "0, 0, 0"))
  (|CallParentFunction CrosshairLocation)
  (if (Variables|Default|GetcanShoot?)
    (CallFunction|ShootProjectile)))

(fn ConstructionScript
  (|CallParentFunction))

(fn SpawningProjectile
  (params (spawnTransform :type Transform))
  (Game|SpawnActorfromClass "/Game/Weapons/BP_ProjectileWind.BP_ProjectileWind_C" spawnTransform "Undefined" self (Variables|Default|GethurricaneDespawnTimer) (Variables|Default|GethurricaneAoeRange) (Variables|Default|GetCrosshairLocation) (Game|GetInstigator)))

(fn ActivateAOE
  (|CallParentFunction)
  (for _array_element (Collision|GetOverlappingActors (Variables|Default|GetSphere) "/Game/Weapons/BP_CollisionBase.BP_CollisionBase_C" :!class /Script/Engine.PrimitiveComponent)
    (bind _asbp_collision_base (Utilities|Casting|CastToBP_CollisionBase _array_element))
    (Default|Knockback _asbp_collision_base (Transformation|GetActorLocation (Game|GetPlayerCharacter 0)) (Variables|Default|GetAreaOfEffectSize) (Variables|Default|GetknockbackStrength)))
  (Components|Sphere|SetSphereRadius (Variables|Default|GetSphere) 0.0 false))