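; Fire staff weapon that fires projectiles on primary shoot and a fire stream on secondary shoot, extending a parent weapon class.
; When shooting is allowed, inherited shoot functions run, and projectile spawning passes base and damage-over-time values to BP_ProjectileFire.
; The stream's hit result applies fire damage over time to BP_CollisionBase actors.
; Stream effects also activate the player's Fire component.
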(event EventOnSecondaryShoot
  (params (CrosshairLocation :type Vector :default "0, 0, 0"))
  (|CallParentFunction CrosshairLocation)
  (if (Variables|Default|GetcanShoot?)
    (bind _hit_results (CallFunction|ShootStream))
    (CallFunction|FireStream _hit_results)))

(event EventOnShoot
  (params (CrosshairLocation :type Vector :default "0, 0, 0"))
  (|CallParentFunction CrosshairLocation)
  (if (Variables|Default|GetcanShoot?)
    (CallFunction|ShootProjectile)))

(fn ConstructionScript
  (|CallParentFunction))

(fn SpawningProjectile
  (params (spawnTransform :type Transform))
  (Game|SpawnActorfromClass "/Game/Weapons/BP_ProjectileFire.BP_ProjectileFire_C" spawnTransform "Undefined" self (Variables|Default|GetfireStreamDamage) (Variables|Default|GetfireDoTDuration) (Variables|Default|GetbaseDamage) (Game|GetInstigator)))

(fn FireStream
  (params (Hit%20result :type Hit%20Result%20Structure))
  (bind _asbp_collision_base (Utilities|Casting|CastToBP_CollisionBase (.HitActor (Collision|BreakHitResult Hit%20result))))
  (Default|OnDoT _asbp_collision_base (Variables|Default|GetfireStreamDamage) (Variables|Default|GetfireDoTDuration) true false))

(fn PlayStreamEffects
  (|CallParentFunction)
  (Components|Activation|Activate (Variables|/Game/Character/EvilBunCharacter.EvilBunCharacter_C|GetFire (Variables|Default|GetPlayer)) false))