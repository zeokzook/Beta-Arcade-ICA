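; Base enemy actor that tracks health and reacts to elemental weapon effects, awarding score on death.
; Damage-over-time timers drive burning and freeze buildup, and basic hits on burning or frozen enemies deal bonus damage.
; Lightning recursively chains to nearby instances, while wind stuns by levitating or launches enemies with distance-scaled knockback that damages on static mesh impacts.
; Tick syncs particles and beams and locks rotation while stunned or frozen.
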(event OnComponentHit(CapsuleComponent)
  (params (HitComponent :type Primitive%20Component%20Object%20Reference) (OtherActor :type Actor%20Object%20Reference) (OtherComp :type Primitive%20Component%20Object%20Reference) (NormalImpulse :type Vector :default "0, 0, 0") (Hit :type Hit%20Result%20Structure%20%28by%20ref%29))
  (bind _self self)
  ;[1 1 1] Wall hit damage from wind staff knockback
  (if (Variables|Default|Getknocked)
    (Utilities|Casting|CastToStaticMeshActor OtherActor)
    (Game|Damage|ApplyDamage _self (* 15.0 (Variables|Default|GetdmgModifier)) (Game|GetInstigatorController) _self)
    (Utilities|IsValid self
      (:Is%20Valid
        (Variables|Default|Setknocked false)
        (Variables|/Script/Engine.CharacterMovementComponent|SetMaxWalkSpeed (Variables|Character|GetCharacterMovement) (Variables|Default|GetinitWalkSpeed))))))

(event Custom|onDoT
  (params (overTimeDmg :type Float%20%28single-precision%29) (overTimeDuration :type Float%20%28single-precision%29) (Fire :type Boolean) (Ice :type Boolean))
  ;[1 1 1] Damage Over Time
  (Variables|Default|SetoverTimeDamage overTimeDmg)
  (Variables|Default|SetoverTimeDuration overTimeDuration)
  (Variables|Default|SetonFire Fire)
  (Variables|Default|SetonIce Ice)
  (CallFunction|DamageOverT)
  (bind _returnvalue (Utilities|Time|SetTimerbyFunctionName 0 "DamageOverT" (Variables|Default|GetoverTimeTick) true))
  (if (Utilities|Time|IsTimerActivebyHandle (stale _returnvalue_2))
    (Utilities|Time|ClearandInvalidateTimerbyHandle (stale _returnvalue_2)))
  (bind _returnvalue_2 (Utilities|Time|SetTimerbyEvent (delegate Custom|notOnDoT) (Variables|Default|GetoverTimeDuration))))

(event Custom|notOnDoT
  ;[1 1 1] Damage Over Time
  (Variables|Default|SetonFire false)
  (Variables|Default|SetonIce false)
  (Utilities|Time|ClearandInvalidateTimerbyHandle (stale Custom|onDoT _returnvalue)))

(event Custom|Electric
  (params (ChainNum :type Integer) (Damage :type Float%20%28single-precision%29) (PreviousActor :type Object%20Object%20Reference) (ChainAll :type Boolean))
  (bind _self self)
  ;[1 1 1] Chain Lightning
  (Utilities|IsValid PreviousActor
    (:Is%20Valid
      (Variables|Default|SetpreviousActor PreviousActor))
    (:Is%20Not%20Valid
      _))
  (if (not (== ChainNum 3))
    (Variables|Default|SetcurrentChainNumber ChainNum)
    (Variables|Default|SetinitialDamage Damage)
    (bind _outactors (Actor|GetAllActorsOfClass "BP_CollisionBase_C"))
    (bind _array_element (Utilities|Array|ForEachLoopwithBreak _outactors :!label _label)
      (:LoopBody
        (if (not (== _array_element _self))
          (if (not (== _array_element (Variables|Default|GetpreviousActor)))
            (if (<= (Math|Vector|Distance(Vector) (Transformation|GetActorLocation _self) (Transformation|GetActorLocation _array_element)) (Variables|Default|GetchainRange))
              (Variables|Default|SetchainedActor _array_element)
              (CallFunction|ActivateChain ChainAll)
              (if (not ChainAll)
                (Development|PrintString "Found nearby enemy!")
                (goto _label Break)))))))))

(event Custom|Stunned
  (params (StunDuration :type Float%20%28single-precision%29))
  (bind _charactermovement (Variables|Character|GetCharacterMovement))
  ;[1 1 1] Wind Staff stunning and knockback
  (Variables|/Script/Engine.CharacterMovementComponent|SetMaxWalkSpeed _charactermovement 0.0)
  (CallFunction|StartStunnedEffect)
  (Utilities|FlowControl|RetriggerableDelay StunDuration)
  (Variables|/Script/Engine.CharacterMovementComponent|SetMaxWalkSpeed _charactermovement (Variables|Default|GetinitWalkSpeed))
  (CallFunction|EndStunnedEffect))

(event Custom|ActivateChain
  (params (ChainAll :type Boolean))
  ;[1 1 1] Chain Lightning
  (if ChainAll
    (Utilities|FlowControl|Delay 0.5)
    (Variables|Default|Setchained true)
    (Variables|Default|SetchainDamage (* (Variables|Default|GetinitialDamage) 0.1))
    (Game|Damage|ApplyDamage (Variables|Default|GetchainedActor) (Variables|Default|GetchainDamage) (Game|GetInstigatorController) self "/Game/Weapons/DamageTypes/DmgType_Lightning.DmgType_Lightning_C" :!label _label)
    (bind _asbp_collision_base (Utilities|Casting|CastToBP_CollisionBase (Variables|Default|GetchainedActor)))
    (Utilities|IsValid _asbp_collision_base
      (:Is%20Valid
        (CallFunction|Electric _asbp_collision_base (Variables|Default|GetcurrentChainNumber) (Variables|Default|GetinitialDamage) self ChainAll)
        (Utilities|FlowControl|Delay 0.2)
        (Variables|Default|Setchained false)))
    (else
      (if (> (Variables|Default|GetcurrentChainNumber) 0)
        (Utilities|FlowControl|Delay 0.5))
      (if (Math|Random|RandomBoolwithWeight 0.5)
        (Variables|Default|Setchained true)
        (switch int (Variables|Default|GetcurrentChainNumber)
          (:0
            (Variables|Default|SetchainDamage (* (Variables|Default|GetinitialDamage) 0.3))
            (Math|Integer|IncrementInt (Variables|Default|GetcurrentChainNumber)
              (:%20%20
                (goto _label))))
          (:1
            (Variables|Default|SetchainDamage (* (Variables|Default|GetinitialDamage) 0.2))
            (Math|Integer|IncrementInt (Variables|Default|GetcurrentChainNumber)
              (:%20%20
                (goto _label))))
          (:2
            (Variables|Default|SetchainDamage (* (Variables|Default|GetinitialDamage) 0.1))
            (Math|Integer|IncrementInt (Variables|Default|GetcurrentChainNumber)
              (:%20%20
                (goto _label)))))))))

(event Custom|Knockback
  (params (PlayerLoc :type Vector) (AOERadius :type Float%20%28single-precision%29) (KnockbackStrength :type Float%20%28single-precision%29))
  (bind _returnvalue (Transformation|GetActorLocation))
  (bind _returnvalue_2 (* AOERadius 2.4))
  (bind _returnvalue_3 (Math|Vector|GetUnitDirection(Vector) PlayerLoc _returnvalue))
  (bind _returnvalue_4 (Math|Vector|Distance(Vector) PlayerLoc _returnvalue))
  (bind _returnvalue_5 (/ _returnvalue_2 _returnvalue_4))
  (bind _returnvalue_6 (* KnockbackStrength _returnvalue_5))
  (bind _returnvalue_7 (* _returnvalue_3 _returnvalue_6))
  ;[1 1 1] Wind Staff stunning and knockback
  (if (not (Variables|Default|Getknocked))
    (Variables|/Script/Engine.CharacterMovementComponent|SetMaxWalkSpeed (Variables|Character|GetCharacterMovement) 0.0)
    (Variables|Default|SetdmgModifier _returnvalue_5)
    (Character|LaunchCharacter (Math|Vector|MakeVector (.x _returnvalue_7) (.y _returnvalue_7) 2.5e+02) false false)
    (Variables|Default|Setknocked true)))

(event Custom|Slow
  ;[1 1 1] Freezing and Slow
  (Variables|/Script/Engine.CharacterMovementComponent|SetMaxWalkSpeed (Variables|Character|GetCharacterMovement) (* (Variables|Default|GetinitWalkSpeed) 0.3)))

(event Custom|End%20Slow
  ;[1 1 1] Freezing and Slow
  (if (not (Variables|Default|GetFrozen))
    (Variables|/Script/Engine.CharacterMovementComponent|SetMaxWalkSpeed (Variables|Character|GetCharacterMovement) (Variables|Default|GetinitWalkSpeed))))

(event Custom|Freezing
  ;[1 1 1] Freezing and Slow
  (if (not (Variables|Default|GetFrozen))
    (bind _result (Math|Float|IncrementFloat (Variables|Default|GetFreeze))
      (:%20%20
        (if (== _result (Variables|Default|GetFreezingPoint))
          (Development|PrintString "Frozen")
          (Utilities|IsValid self
            (:Is%20Valid
              (Variables|Default|SetFrozen true)
              (Variables|/Script/Engine.CharacterMovementComponent|SetMaxWalkSpeed (Variables|Character|GetCharacterMovement) 0.0)
              (Variables|Default|SetcurrentRotation (Transformation|GetWorldRotation (Variables|Collision|GetCapsuleComponent)))
              (bind _returnvalue (Utilities|Time|SetTimerbyFunctionName 0 "ClearFrozen" 0.5 true :!label _label))
              (Variables|Default|SetFrozenTimerHandle _returnvalue)))
          (else
            (Development|PrintString "Freezing")
            (Utilities|FlowControl|RetriggerableDelay 1.0)
            (if (not (Variables|Default|GetFrozen))
              (goto _label))))))))

(event EventBeginPlay
  (Variables|Default|SetinitWalkSpeed (Variables|/Script/Engine.CharacterMovementComponent|GetMaxWalkSpeed (Variables|Character|GetCharacterMovement)))
  (Variables|Default|SetHealth (Variables|Default|GetmaxHealth))
  (Components|Activation|Deactivate (Variables|Default|GetFire))
  (Components|Activation|Deactivate (Variables|Default|GetLightning))
  (Components|Activation|Deactivate (Variables|Default|GetIce))
  ;[1 1 1] Enemy Health bar
  (bind _asenemy_health_bar (Utilities|Casting|CastToEnemyHealthBar (UserInterface|GetUserWidgetObject (Variables|Default|GetHealthbar))))
  (Variables|Default|SetEnemyHealthBar _asenemy_health_bar)
  (Variables|/Game/Weapons/EnemyHealthBar.EnemyHealthBar_C|SetOwner _asenemy_health_bar self))

(event EventTick
  (params (DeltaSeconds :type Float%20%28single-precision%29))
  (Utilities|FlowControl|Sequence
    (:then_0
      ;[1 1 1] Particle system controls
      (if (Variables|Default|GetonFire)
        (CallFunction|BeginFireParticles)
        (else
          (CallFunction|EndFireParticles))))
    (:then_1
      (if (Variables|Default|Getchained)
        (CallFunction|BeginElectricBeam)
        (else
          (CallFunction|EndElectricBeam))))
    (:then_2
      ;[1 1 1] Wall hit damage from wind staff knockback
      (if (Variables|Default|Getknocked)
        (if (not (AI|Components|NavMovement|IsFalling (Variables|Character|GetCharacterMovement)))
          (Utilities|IsValid self
            (:Is%20Valid
              (Variables|Default|Setknocked false)
              (Variables|/Script/Engine.CharacterMovementComponent|SetMaxWalkSpeed (Variables|Character|GetCharacterMovement) (Variables|Default|GetinitWalkSpeed)))))))
    (:then_3
      (if (Variables|Default|GetFrozen)
        (Transformation|SetActorRotation (Variables|Default|GetcurrentRotation) true :!label _label)))
    (:then_4
      (if (Variables|Default|Getstun)
        (goto _label)))
    (:then_5
      (if (> (Variables|Default|GetFreeze) 0.0)
        (CallFunction|BeginIceParticles)
        (else
          (CallFunction|EndIceParticles))))))

(event Game|Damage|EventAnyDamage
  (params (Damage :type Float%20%28single-precision%29) (DamageType :type Damage%20Type%20Object%20Reference) (InstigatedBy :type Controller%20Object%20Reference) (DamageCauser :type Actor%20Object%20Reference))
  (bind _mesh (Variables|Character|GetMesh))
  (if (== (Utilities|GetClass DamageType) "/Game/Weapons/DamageTypes/DmgType_Basic.DmgType_Basic_C")
    (if (Variables|Default|GetonFire)
      ;[1 1 1] More damage when basic bullet hits enemy on Fire/Ice
      (Variables|Default|SetHealth (- (Variables|Default|GetHealth) (* Damage 1.5)) :!label _label)
      (if (Variables|Default|GetFrozen)
        (Variables|Default|SetFrozen false)
        (Variables|/Script/Engine.CharacterMovementComponent|SetMaxWalkSpeed (Variables|Character|GetCharacterMovement) (Variables|Default|GetinitWalkSpeed))
        (Utilities|Time|ClearandInvalidateTimerbyHandle (Variables|Default|GetFrozenTimerHandle))
        (Variables|Default|SetFreeze 0.0)
        (CallFunction|NotonDoT))
      (elif (Variables|Default|GetFrozen)
        (goto _label)
        (else
          ;[1 1 1] Normal Damage
          (Variables|Default|SetHealth (- (Variables|Default|GetHealth) Damage) :!label _label_2))))
    (else
      (goto _label_2)))
  (CallFunction|CheckDeath)
  (Utilities|IsValid self
    (:Is%20Valid
      ;[1 1 1] Flashing red when damaged
      (Rendering|Material|SetVectorParameterValueonMaterials _mesh "BodyColor" "0.850980,0.039215,0.039215")
      (Utilities|FlowControl|Delay 0.2)
      (Rendering|Material|SetVectorParameterValueonMaterials _mesh "BodyColor" "0.450980,0.403922,0.360784")
      (Development|PrintString (Utilities|String|BuildString(Float) "" "Mob Health: " (Variables|Default|GetHealth)) true true "(R=1.000000,G=0.058824,B=0.000000,A=1.000000)"))))

(fn ConstructionScript)

(fn DamageOverT
  (Game|Damage|ApplyDamage self (Variables|Default|GetoverTimeDamage) 0 0)
  (if true
    (CallFunction|Freezing)))

(fn BeginFireParticles
  (Utilities|IsValid self
    (:Is%20Valid
      (Components|Activation|Activate (Variables|Default|GetFire) false))))

(fn EndFireParticles
  (Utilities|IsValid self
    (:Is%20Valid
      (Components|Activation|Deactivate (Variables|Default|GetFire)))))

(fn CheckDeath
  (if (<= (Variables|Default|GetHealth) 0.0)
    (if (== (Math|Random|RandomInteger 10) 10)
      (Game|SpawnActorfromClass "/Game/Pickups/NukePickup.NukePickup_C" (Transformation|GetActorTransform) "Undefined" 0 0))
    (Actor|DestroyActor)
    (Development|PrintString "Enemy Dead")
    (CallFunction|AddScore)))

(fn AddScore
  (bind _asevil_bun_controller (Utilities|Casting|CastToEvilBunController (Game|GetPlayerController 0)))
  (if (Utilities|Enum|Equal(Enum) (Variables|Default|GetName) "NewEnumerator0")
    (Variables|/Game/Character/EvilBunController.EvilBunController_C|SetScore _asevil_bun_controller (+ (Variables|/Game/Character/EvilBunController.EvilBunController_C|GetScore _asevil_bun_controller) (Variables|Default|GetScoreAmount)))
    (Development|PrintString (Utilities|String|BuildString(Integer) "" "Score: " (Variables|/Game/Character/EvilBunController.EvilBunController_C|GetScore _asevil_bun_controller)) :!label _label)
    (elif (Utilities|Enum|Equal(Enum) (Variables|Default|GetName) "NewEnumerator1")
      (Variables|/Game/Character/EvilBunController.EvilBunController_C|SetScore _asevil_bun_controller (+ (Variables|/Game/Character/EvilBunController.EvilBunController_C|GetScore _asevil_bun_controller) (Variables|Default|GetScoreAmount)))
      (goto _label))))

(fn BeginElectricBeam
  (bind _chainedactor (Variables|Default|GetchainedActor))
  (bind _lightning (Variables|Default|GetLightning))
  (Utilities|IsValid self
    (:Is%20Valid
      (Utilities|IsValid _chainedactor
        (:Is%20Valid
          (Niagara|SetNiagaraVariable(Vector3) _lightning "beamStart" (Transformation|GetActorLocation))
          (Niagara|SetNiagaraVariable(Vector3) _lightning "beamEnd" (Transformation|GetActorLocation _chainedactor))
          (Components|Activation|Activate _lightning true))))))

(fn EndElectricBeam
  (Utilities|IsValid self
    (:Is%20Valid
      (Components|Activation|Deactivate (Variables|Default|GetLightning)))))

(fn StartStunnedEffect
  (bind _returnvalue (Transformation|GetActorLocation))
  (Transformation|SetActorLocation (Math|Vector|MakeVector (.x _returnvalue) (.y _returnvalue) (+ (.z _returnvalue) 5e+01)) true false)
  (Variables|/Script/Engine.CharacterMovementComponent|SetGravityScale (Variables|Character|GetCharacterMovement) 0.0)
  (Variables|Default|SetcurrentRotation (Transformation|GetWorldRotation (Variables|Collision|GetCapsuleComponent)))
  (Variables|Default|Setstun true))

(fn EndStunnedEffect
  (Variables|/Script/Engine.CharacterMovementComponent|SetGravityScale (Variables|Character|GetCharacterMovement) 1.0)
  (Variables|Default|Setstun false))

(fn ClearFrozen
  (Development|PrintString "Unfreezing")
  (if (Variables|Default|GetFrozen)
    (bind _output_get (Variables|Default|SetFreeze (Math|Float|Clamp(Float) (- (Variables|Default|GetFreeze) 2.5) 0.0 (Variables|Default|GetFreezingPoint))))
    (if (<= _output_get 0.0)
      (Variables|Default|SetFrozen false)
      (Variables|/Script/Engine.CharacterMovementComponent|SetMaxWalkSpeed (Variables|Character|GetCharacterMovement) (Variables|Default|GetinitWalkSpeed))
      (Utilities|Time|ClearandInvalidateTimerbyHandle (Variables|Default|GetFrozenTimerHandle))
      (CallFunction|NotonDoT)
      (Variables|Default|SetFreeze 0.0))
    (else
      (Variables|Default|SetFreeze (Math|Float|Clamp(Float) (- (Variables|Default|GetFreeze) 1.0) 0.0 (Variables|Default|GetFreezingPoint)))
      (if (<= (Variables|Default|GetFreeze) 0.0)
        (Variables|Default|SetFreeze 0.0)
        (Utilities|Time|ClearandInvalidateTimerbyHandle (Variables|Default|GetFrozenTimerHandle))))))

(fn BeginIceParticles
  (Utilities|IsValid self
    (:Is%20Valid
      (Components|Activation|Activate (Variables|Default|GetIce) false))))

(fn EndIceParticles
  (Utilities|IsValid self
    (:Is%20Valid
      (Components|Activation|Deactivate (Variables|Default|GetIce)))))